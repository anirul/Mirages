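; Player character for a click-to-move game with 2D flipbook visuals and a draining life timer.
; Each tick it shows the idle flipbook when stationary, otherwise picks one of four walk flipbooks from the direction toward the controller's clicked location, and zeroes mesh rotation as billboarding.
; Life counts down alongside an elapsed-time counter, opening the credits level when exhausted.
; AnyDamage adds to life, capped at a maximum, acting as healing.
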(event EventAnyDamage
  (params (Damage :type Float%20%28single-precision%29) (DamageType :type Damage%20Type%20Object%20Reference) (InstigatedBy :type Controller%20Object%20Reference) (DamageCauser :type Actor%20Object%20Reference))
  ;[1 1 1] Increment life
  (if (> (+ Damage (Variables|Default|GetTotalLife)) 1e+02)
    (Variables|Default|SetTotalLife 1e+02)
    (else
      (Variables|Default|SetTotalLife (+ Damage (Variables|Default|GetTotalLife))))))

(event EventTick
  (params (DeltaSeconds :type Float%20%28single-precision%29))
  (bind _returnvalue (Transformation|GetActorLocation))
  ;[1 1 1] Check if moving
  (Variables|Default|SetdetlaTime DeltaSeconds)
  ;[1 1 1] Get vector direction of character
  (bind _asmy_controller (Utilities|Casting|CastToMyController (Game|GetPlayerController 0)))
  (if (Math|Vector|Equal(Vector) (Variables|Default|GetplayerLocation) _returnvalue 0.0001)
    ;[1 1 1] not moving
    (Rendering|SetVisibility (Variables|Default|GetFlipbookIdleFront) true false)
    (Rendering|SetVisibility (Variables|Default|GetFlipbookWalkRight) false false)
    (else
      (Variables|Default|SetplayerLocation _returnvalue)
      ;[1 1 1] moving so no idle
      (Rendering|SetVisibility (Variables|Default|GetFlipbookIdleFront) false false)
      ;[1 1 1] Activate correct direction
      (Rendering|SetVisibility (Variables|Default|GetFlipbookWalkBack) (and (> (.X (Math|Vector|BreakVector (Class|KismetMathLibrary|GetDirectionVector (Transformation|GetActorLocation) (Variables|/Game/Blueprints/MyController.MyController_C|GetclicLocation _asmy_controller)))) (.Y (Math|Vector|BreakVector (Class|KismetMathLibrary|GetDirectionVector (Transformation|GetActorLocation) (Variables|/Game/Blueprints/MyController.MyController_C|GetclicLocation _asmy_controller))))) (> (.X (Math|Vector|BreakVector (Class|KismetMathLibrary|GetDirectionVector (Transformation|GetActorLocation) (Variables|/Game/Blueprints/MyController.MyController_C|GetclicLocation _asmy_controller)))) (* (.Y (Math|Vector|BreakVector (Class|KismetMathLibrary|GetDirectionVector (Transformation|GetActorLocation) (Variables|/Game/Blueprints/MyController.MyController_C|GetclicLocation _asmy_controller)))) -1.0))) false)
      (Rendering|SetVisibility (Variables|Default|GetFlipbookWalkFront) (and (not (> (.X (Math|Vector|BreakVector (Class|KismetMathLibrary|GetDirectionVector (Transformation|GetActorLocation) (Variables|/Game/Blueprints/MyController.MyController_C|GetclicLocation _asmy_controller)))) (.Y (Math|Vector|BreakVector (Class|KismetMathLibrary|GetDirectionVector (Transformation|GetActorLocation) (Variables|/Game/Blueprints/MyController.MyController_C|GetclicLocation _asmy_controller)))))) (not (> (.X (Math|Vector|BreakVector (Class|KismetMathLibrary|GetDirectionVector (Transformation|GetActorLocation) (Variables|/Game/Blueprints/MyController.MyController_C|GetclicLocation _asmy_controller)))) (* (.Y (Math|Vector|BreakVector (Class|KismetMathLibrary|GetDirectionVector (Transformation|GetActorLocation) (Variables|/Game/Blueprints/MyController.MyController_C|GetclicLocation _asmy_controller)))) -1.0)))) false)
      (Rendering|SetVisibility (Variables|Default|GetFlipbookWalkLeft) (and (> (.X (Math|Vector|BreakVector (Class|KismetMathLibrary|GetDirectionVector (Transformation|GetActorLocation) (Variables|/Game/Blueprints/MyController.MyController_C|GetclicLocation _asmy_controller)))) (.Y (Math|Vector|BreakVector (Class|KismetMathLibrary|GetDirectionVector (Transformation|GetActorLocation) (Variables|/Game/Blueprints/MyController.MyController_C|GetclicLocation _asmy_controller))))) (not (> (.X (Math|Vector|BreakVector (Class|KismetMathLibrary|GetDirectionVector (Transformation|GetActorLocation) (Variables|/Game/Blueprints/MyController.MyController_C|GetclicLocation _asmy_controller)))) (* (.Y (Math|Vector|BreakVector (Class|KismetMathLibrary|GetDirectionVector (Transformation|GetActorLocation) (Variables|/Game/Blueprints/MyController.MyController_C|GetclicLocation _asmy_controller)))) -1.0)))) false)
      (Rendering|SetVisibility (Variables|Default|GetFlipbookWalkRight) (and (not (> (.X (Math|Vector|BreakVector (Class|KismetMathLibrary|GetDirectionVector (Transformation|GetActorLocation) (Variables|/Game/Blueprints/MyController.MyController_C|GetclicLocation _asmy_controller)))) (.Y (Math|Vector|BreakVector (Class|KismetMathLibrary|GetDirectionVector (Transformation|GetActorLocation) (Variables|/Game/Blueprints/MyController.MyController_C|GetclicLocation _asmy_controller)))))) (> (.X (Math|Vector|BreakVector (Class|KismetMathLibrary|GetDirectionVector (Transformation|GetActorLocation) (Variables|/Game/Blueprints/MyController.MyController_C|GetclicLocation _asmy_controller)))) (* (.Y (Math|Vector|BreakVector (Class|KismetMathLibrary|GetDirectionVector (Transformation|GetActorLocation) (Variables|/Game/Blueprints/MyController.MyController_C|GetclicLocation _asmy_controller)))) -1.0))) false)))
  ;[1 1 1] billboard the character
  (Transformation|SetWorldRotation (Variables|Character|GetMesh) "0,0.000000, 0" false)
  ;[1 1 1] Decrement life Increment time
  (Variables|Default|SetTotalLife (- (Variables|Default|GetTotalLife) (Variables|Default|GetdetlaTime)))
  (Variables|Default|SetTotalTime (+ (Variables|Default|GetdetlaTime) (Variables|Default|GetTotalTime)))
  ;[1 1 1] Death
  (if (<= (- (Variables|Default|GetTotalLife) (Variables|Default|GetdetlaTime)) 0.0)
    (Game|OpenLevel(byName) "credits")))

(fn ConstructionScript
  ;[1 1 1] Set the begin of time of life
  (Variables|Default|SetTotalLife 6e+01)
  (Variables|Default|SetTotalTime 0.0)
  ;[1 1 1] set default flipbook to idle front
  (Rendering|SetVisibility (Variables|Default|GetFlipbookWalkFront) false false)
  (Rendering|SetVisibility (Variables|Default|GetFlipbookIdleFront) true false))